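; Player camera actor that becomes the first player controller's view target and follows the player character's location.
; BeginPlay applies the configured boom length, actor rotation and FOV, then links itself and PlayerCharacter_BP through mutual references.
; The FollowPlayer timeline serves as the update loop, snapping the actor to the player's location while start and stop events toggle following.
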(event `self.ReceiveBeginPlay`
  ;[1 1 1] ConfigCamera
  (`PlayerController.SetViewTargetWithBlend` (`GameplayStatics.GetPlayerController` 0) self 0.0 "VTBlend_Linear" 0.0 false)
  (set `SpringArmComponent.TargetArmLength` (`self.Camera_ArmLength`) (`self.CameraBoom`))
  (`self.K2_SetActorRotation` (`self.Camera_ArmRotation`))
  (`CameraComponent.SetFieldOfView` (`self.Camera`) (`self.Camera_FOV`))
  (bind _asplayer_character_bp (cast `/Game/Blueprints/PlayerBP/PlayerCharacter_BP` (`GameplayStatics.GetPlayerCharacter` 0)))
  (bind _output_get (set `self.PlayerReference` _asplayer_character_bp))
  (set `/Game/Blueprints/PlayerBP/PlayerCharacter_BP.CameraReference` self _output_get)
  (`self.StartFollowingPlayer`))

(event `StartFollowingPlayer`
  ;[1 1 1] MoveCamera
  (`/Engine/EditorBlueprintResources/StandardMacros.IsValid` (`self.PlayerReference`)
    (:`Is Valid`
      (`Timeline|FollowPlayer` :!label _label
        (:`Update`
          (`self.K2_SetActorLocation` (`self.K2_GetActorLocation` (`self.PlayerReference`))))))))

(event `StopFollowingPlayer`
  ;[1 1 1] MoveCamera
  (goto _label :!via `Stop`))

(fn `UserConstructionScript`)