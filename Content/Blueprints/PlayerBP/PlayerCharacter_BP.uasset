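; Player character Blueprint with camera-relative movement, jumping and a landing indicator shown while airborne.
; Movement axes follow the referenced camera actor's yaw and smoothly turn control rotation toward horizontal velocity.
; CameraTurn input adjusts that camera's yaw within a clamped arc.
; While falling, a downward sphere trace sets the indicator's height just above the hit surface, or drops it far down on a miss.
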(event `InputAxis|MoveForward`
  (params (AxisValue :type "Float (single-precision)"))
  (bind _returnvalue (`GameplayStatics.GetPlayerController` 0))
  (bind (_returnvalue_roll _returnvalue_pitch _returnvalue_yaw) (`KismetMathLibrary.BreakRotator` (`self.K2_GetActorRotation` (`self.CameraReference`))))
  (bind _returnvalue_2 (* (`self.GetVelocity`) (1.0 1.0 0.0)))
  (`self.AddMovementInput` (`KismetMathLibrary.GetForwardVector` (`KismetMathLibrary.MakeRotator` 0.0 0.0 _returnvalue_yaw)) AxisValue)
  (if (!= _returnvalue_2 (0.0 0.0 0.0)) :!label _label
    (`Controller.SetControlRotation` _returnvalue (`KismetMathLibrary.RInterpTo` (`Controller.GetControlRotation` _returnvalue) (`KismetMathLibrary.MakeRotFromX` _returnvalue_2) (`GameplayStatics.GetWorldDeltaSeconds`) 5.0))))

(event `InputAxis|MoveRight`
  (params (AxisValue :type "Float (single-precision)"))
  (bind (_returnvalue_roll _returnvalue_pitch _returnvalue_yaw) (`KismetMathLibrary.BreakRotator` (`self.K2_GetActorRotation` (`self.CameraReference`))))
  (`self.AddMovementInput` (`KismetMathLibrary.GetRightVector` (`KismetMathLibrary.MakeRotator` 0.0 0.0 _returnvalue_yaw)) AxisValue)
  (goto _label))

(event `InputAxis|CameraTurn`
  (params (AxisValue :type "Float (single-precision)"))
  (bind _camerareference (`self.CameraReference`))
  (bind (_camera_armrotation_roll _camera_armrotation_pitch _camera_armrotation_yaw) (`KismetMathLibrary.BreakRotator` (`/Game/Blueprints/PlayerBP/PlayerCamera_BP.Camera_ArmRotation` _camerareference)))
  (`/Engine/EditorBlueprintResources/StandardMacros.IsValid` _camerareference
    (:`Is Valid`
      (bind _output_get (set `/Game/Blueprints/PlayerBP/PlayerCamera_BP.Camera_ArmRotation` (`KismetMathLibrary.MakeRotator` _camera_armrotation_roll _camera_armrotation_pitch (`KismetMathLibrary.ClampAngle` (+ (* AxisValue (`/Game/Blueprints/PlayerBP/PlayerCamera_BP.Camera_TurnSpeed` _camerareference)) _camera_armrotation_yaw) -45.0 45.0)) _camerareference))
      (`self.K2_SetActorRotation` (`self.CameraReference`) _output_get false))))

(event `InputAction|Jump`
  (params (Key :type "Key Structure"))
  (:`Pressed`
    (`self.Jump`)))

(event `self.ReceiveTick`
  (params (DeltaSeconds :type "Float (single-precision)"))
  (`self.LandingIndicator_Display`))

(event `LandingIndicator_Display`
  (bind _returnvalue (`self.K2_GetActorLocation`))
  (bind _landingindicator (`self.LandingIndicator`))
  (bind _landingindicator_2 (`self.LandingIndicator`))
  (bind (_returnvalue_x _returnvalue_y _returnvalue_z) (`KismetMathLibrary.BreakVector` (`SceneComponent.K2_GetComponentLocation` _landingindicator)))
  (if (`NavMovementComponent.IsFalling` (`self.CharacterMovement`))
    (`SceneComponent.SetVisibility` _landingindicator_2 true false)
    (bind (_outhit _returnvalue_2) (`KismetSystemLibrary.SphereTraceSingle` _returnvalue (+ _returnvalue (0.0 0.0 -3200.0)) 36.0 "TraceTypeQuery1"))
    (if _returnvalue_2
      (`SceneComponent.K2_SetWorldLocation` _landingindicator (+ (`KismetMathLibrary.MakeVector` _returnvalue_x _returnvalue_y (.z (`.ImpactPoint` (`GameplayStatics.BreakHitResult` _outhit)))) (0.0 0.0 1.0)) false false)
      (else
        (`SceneComponent.K2_SetWorldLocation` _landingindicator (+ (`KismetMathLibrary.MakeVector` _returnvalue_x _returnvalue_y _returnvalue_z) (0.0 0.0 -3199.0)) false false)))
    (else
      (`SceneComponent.SetVisibility` _landingindicator_2 false false))))

(fn `UserConstructionScript`)